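; PC_Test is a test player controller that shows the mouse cursor and drives a measurement tool.
; The 1 key toggles the tool by spawning a BP_Tool_Measure actor or destroying the existing one.
; Left clicks are forwarded to the tool's active measure type actor, handled only when it casts to the linear measure Blueprint.
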(event EventBeginPlay
  (Variables|Default|SetbShowMouseCursor true))

(event EventTick
  (params (DeltaSeconds :type Float%20%28single-precision%29)))

(event Input|KeyboardEvents|1
  (params (Key :type Key%20Structure :default "None"))
  (:Pressed
    (bind _measuretool (Variables|Default|GetMeasureTool)
      (:then
        (Actor|DestroyActor _measuretool)
        (Variables|Default|SetMeasureTool 0))
      (:else
        (bind _returnvalue (Game|SpawnActorfromClass "/Game/Project/02_Blueprints/Measure/BP_Tool_Measure.BP_Tool_Measure_C" (Math|Transform|MakeTransform "0, 0, 0" "0, 0, 0" "1.000000,1.000000,1.000000") "Undefined" "MultiplyWithRoot" 0 0))
        (Variables|Default|SetMeasureTool _returnvalue)))))

(event Input|MouseEvents|LeftMouseButton
  (params (Key :type Key%20Structure :default "None"))
  (bind _measuretool (Variables|Default|GetMeasureTool))
  (bind _measuretypeactor (Variables|/Game/Project/02_Blueprints/Measure/BP_Tool_Measure.BP_Tool_Measure_C|GetMeasureTypeActor _measuretool))
  (:Pressed
    (Utilities|IsValid _measuretool
      (:Is%20Valid
        (Utilities|IsValid _measuretypeactor
          (:Is%20Valid
            (bind _asbp_tool_measure__linear (Utilities|Casting|CastToBP_Tool_Measure-Linear _measuretypeactor))
            (Default|OnLeftMouseClick _asbp_tool_measure__linear)))))))

(fn ConstructionScript)