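; BP_Tool_Measure is the measurement tool actor that manages the selector UI and the active measure-type actor.
; BeginPlay creates the UW_Main widget, links its type selector back to this tool, and Destroyed removes it.
; EnableMeasureType destroys any existing measure actor, or otherwise spawns one for the chosen type; None also destroys it.
; Only linear measuring has an actor class assigned; surface and path are empty.
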(event EventBeginPlay
  (bind _returnvalue (UserInterface|CreateWidget "/Game/Project/02_Blueprints/World/UW_Main.UW_Main_C"))
  (bind _output_get (Variables|Default|SetButtons _returnvalue))
  (Variables|/Game/Project/02_Blueprints/Measure/UW_MeasureTypeSelector.UW_MeasureTypeSelector_C|SetToolMeasure (Variables|/Game/Project/02_Blueprints/World/UW_Main.UW_Main_C|GetUW_MeasureTypeSelector _output_get) self)
  (UserInterface|Viewport|AddtoViewport _returnvalue 0))

(event Collision|EventActorBeginOverlap
  (params (OtherActor :type Actor%20Object%20Reference)))

(event EventTick
  (params (DeltaSeconds :type Float%20%28single-precision%29)))

(event EventDestroyed
  (Widget|RemovefromParent (Variables|Default|GetButtons)))

(fn ConstructionScript)

(fn EnableMeasureType
  (params (MeasureTypes :type E_MeasureTypes%20Enum :default "NewEnumerator0"))
  (bind _output_get (Variables|Default|SetMeasureType MeasureTypes))
  (if (not (Utilities|Enum|Equal(Enum) _output_get "NewEnumerator0"))
    (bind _measuretypeactor (Variables|Default|GetMeasureTypeActor)
      (:then
        (Actor|DestroyActor _measuretypeactor :!label _label)
        (Variables|Default|SetMeasureTypeActor 0))
      (:else
        (bind _returnvalue (Game|SpawnActorfromClass (Utilities|Select :Index _output_get :NewEnumerator0 0 :NewEnumerator1 0 :NewEnumerator2 0 :NewEnumerator3 "/Game/Project/02_Blueprints/Measure/BP_Tool_Measure-Linear.BP_Tool_Measure-Linear_C") (Math|Transform|MakeTransform "0, 0, 0" "0, 0, 0" "1.000000,1.000000,1.000000") "Undefined" "MultiplyWithRoot" 0 0))
        (Variables|Default|SetMeasureTypeActor _returnvalue)))
    (else
      (goto _label))))