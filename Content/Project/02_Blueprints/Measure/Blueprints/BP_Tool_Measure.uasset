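; Measurement tool manager actor that provides the measuring UI and spawns the actor for the selected measure type.
; On BeginPlay it creates the main widget, links itself to its type selector, and adds a cursor image that follows the mouse on a looping timer.
; EnableMeasureType spawns the surface or linear tool (path has no class), or only destroys any existing one.
; On destruction it removes both widgets and the active tool.
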(event Custom|UpdateCursorImageLocation
  ;[1 1 1] Comment
  (bind _returnvalue (Class|WidgetLayoutLibrary|GetMousePositiononViewport))
  (Class|UserWidget|SetPositioninViewport (Variables|Default|GetCursorImage) _returnvalue false))

(event EventBeginPlay
  (bind _returnvalue (UserInterface|CreateWidget "/Game/Project/02_Blueprints/World/UW_Main.UW_Main_C"))
  (bind _output_get (Variables|Default|SetButtons _returnvalue))
  (Variables|/Game/Project/02_Blueprints/Measure/Widgets/UW_MeasureTypeSelector.UW_MeasureTypeSelector_C|SetToolMeasure (Variables|/Game/Project/02_Blueprints/World/UW_Main.UW_Main_C|GetUW_MeasureTypeSelector _output_get) self)
  (UserInterface|Viewport|AddtoViewport _returnvalue 0)
  ;[1 1 1] Comment
  (bind _returnvalue_2 (UserInterface|CreateWidget "/Game/Project/02_Blueprints/Measure/Widgets/UW_CursorImage.UW_CursorImage_C"))
  (bind _output_get_2 (Variables|Default|SetCursorImage _returnvalue_2))
  (Utilities|Time|SetTimerbyEvent (delegate Custom|UpdateCursorImageLocation) 0.01 true)
  (UserInterface|Viewport|AddtoViewport _output_get_2 0))

(event Collision|EventActorBeginOverlap
  (params (OtherActor :type Actor%20Object%20Reference)))

(event EventTick
  (params (DeltaSeconds :type Float%20%28single-precision%29)))

(event EventDestroyed
  (bind _measuretypeactor (Variables|Default|GetMeasureTypeActor))
  (Widget|RemovefromParent (Variables|Default|GetButtons))
  (Utilities|IsValid _measuretypeactor
    (:Is%20Valid
      (Actor|DestroyActor _measuretypeactor))))

(fn ConstructionScript)

(fn EnableMeasureType
  (params (MeasureTypes :type E_MeasureTypes%20Enum :default "NewEnumerator0"))
  (bind _output_get (Variables|Default|SetMeasureType MeasureTypes))
  (if (not (Utilities|Enum|Equal(Enum) _output_get "NewEnumerator0"))
    (bind _measuretypeactor (Variables|Default|GetMeasureTypeActor)
      (:then
        (Actor|DestroyActor _measuretypeactor :!label _label)
        (Variables|Default|SetMeasureTypeActor 0))
      (:else
        (bind _returnvalue (Game|SpawnActorfromClass (Utilities|Select :Index _output_get :NewEnumerator0 0 :NewEnumerator1 "/Game/Project/02_Blueprints/Measure/Blueprints/BP_Tool_Measure-Surface.BP_Tool_Measure-Surface_C" :NewEnumerator2 0 :NewEnumerator3 "/Game/Project/02_Blueprints/Measure/Blueprints/BP_Tool_Measure-Linear.BP_Tool_Measure-Linear_C") (Math|Transform|MakeTransform "0, 0, 0" "0, 0, 0" "1.000000,1.000000,1.000000") "Undefined" "MultiplyWithRoot" 0 0))
        (Variables|Default|SetMeasureTypeActor _returnvalue)))
    (else
      (goto _label))))