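; Surface measuring tool that lets the player place a four-point spline with the mouse and computes the enclosed area.
; Looping timers drive the updates: unplaced points follow the cursor's floor trace, each left click locks the next, and a click after the last restarts.
; Spline meshes and point markers visualize the outline.
; Tick derives segment lengths and sums two Heron's-formula triangles for area, with optional debug overlays.
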(event Custom|UpdateSplineActiveSplinePoint
  ;[1 1 1] Comment
  (for _array_element (Variables|Default|GetPointsToControl)
    (Spline|SetLocationatSplinePoint (Variables|Default|GetSpline) _array_element (Tracing|GetHitLocationMouseonFloor) "Local" true)))

(event Custom|UpdateLineVisuals
  (bind _spline (Variables|Default|GetSpline))
  ;[1 1 1] Comment
  (Utilities|FlowControl|Sequence
    (:then_0
      (for (_array_element _array_index) (Variables|Default|GetSplineMeshComponent)
        (SplineMesh|SetStartandEnd _array_element (.Location (Spline|GetLocationandTangentatSplinePoint _spline _array_index "Local")) (.Tangent (Spline|GetLocationandTangentatSplinePoint _spline _array_index "Local")) (.Location (Spline|GetLocationandTangentatSplinePoint _spline (+ _array_index 1) "Local")) (.Tangent (Spline|GetLocationandTangentatSplinePoint _spline (+ _array_index 1) "Local")) true :!class /Script/Engine.SplineMeshComponent)))
    (:then_1
      (for (_array_element_2 _array_index_2) (Variables|Default|GetMeshComponents)
        (Transformation|SetWorldLocation _array_element_2 (.Location (Spline|GetLocationandTangentatSplinePoint (Variables|Default|GetSpline) _array_index_2 "Local")) false false)))))

(event EventBeginPlay
  (bind _linewidth (Variables|Default|GetLineWidth))
  (bind _returnvalue (Math|Conversions|ToVector2D(Vector) _linewidth))
  (Utilities|FlowControl|Sequence
    (:then_0
      (CallFunction|ResetArray))
    (:then_1
      (Utilities|Time|SetTimerbyEvent (EventDispatchers|CreateEvent :!event Custom|UpdateSplineActiveSplinePoint) 0.01 true))
    (:then_2
      (for _index (range 0 (- (Spline|GetNumberOfSplinePoints (Variables|Default|GetSpline)) 0))
        (Utilities|FlowControl|Sequence
          (:then_0
            ;[1 1 1] Comment
            (bind _returnvalue_2 (AddComponent|AddSplineMeshComponent false))
            (Components|StaticMesh|SetStaticMesh _returnvalue_2 "/Game/Project/02_Blueprints/Measure/Assets/Mesh/MeasureMesh.MeasureMesh")
            (SplineMesh|SetEndScale _returnvalue_2 _returnvalue true :!class /Script/Engine.SplineMeshComponent)
            (SplineMesh|SetStartScale _returnvalue_2 _returnvalue true :!class /Script/Engine.SplineMeshComponent)
            (Utilities|Array|Add (Variables|Default|GetSplineMeshComponent) _returnvalue_2))
          (:then_1
            ;[1 1 1] Comment
            (bind _returnvalue_3 (AddComponent|AddStaticMeshComponent false (Math|Transform|MakeTransform "0, 0, 0" "0, 0, 0" "0.040000,0.040000,0.040000")))
            (Utilities|Array|Add (Variables|Default|GetMeshComponents) _returnvalue_3))))
      (Utilities|Time|SetTimerbyEvent (EventDispatchers|CreateEvent :!event Custom|UpdateLineVisuals) 0.01 true))))

(event EventTick
  (params (DeltaSeconds :type Float%20%28single-precision%29))
  (bind _segment_lengths (SplineSegments|GetAllSplineSegmentsLengths (Variables|Default|GetSpline)))
  (bind _output_get (Variables|Default|SetSegment%20Lengths _segment_lengths))
  (bind _keys (Utilities|Map|Keys _output_get))
  (bind _output_get_2 (Variables|Default|SetSegmentLengths _keys))
  (bind _area_in_m2 (CallFunction|CalculateAreaOfIrregularQuadrilateral (Variables|Default|GetSpline) _output_get_2))
  (Variables|Default|SetTotalArea _area_in_m2)
  ;[1 1 1] Debug Functions
  (if (Variables|Default|GetDebug%20Spline)
    (CallFunction|DebugShowSegmentLengthsonSpline (Variables|Default|GetSegment%20Lengths) (Variables|Default|GetSpline) "NewEnumerator0")
    (CallFunction|DebugShowIndicesonSpline (Variables|Default|GetSpline))
    (CallFunction|DebugShowAreaonSpline (Variables|Default|GetSpline) (Variables|Default|GetTotalArea) "NewEnumerator6")
    (CallFunction|DebugShowMidpointonSpline (Variables|Default|GetSpline) 5e+01)))

(fn ConstructionScript)

(fn GetHitLocationMouseonFloor
  (bind _returnvalue (Game|GetPlayerController 0))
  (bind _hitresult (Game|Player|GetHitResultUnderCursorbyChannel _returnvalue "TraceTypeQuery3" false))
  (bind (_bblockinghit _binitialoverlap _time _distance _location) (Collision|BreakHitResult _hitresult))
  (if _bblockinghit
    (return _location)
    (else
      (return "0.000000,0.000000,-50000.000000"))))

(fn OnLeftClick
  (if (Utilities|Array|IsEmpty (Variables|Default|GetPointsToControl))
    (CallFunction|ResetArray)
    (else
      (Utilities|Array|RemoveIndex (Variables|Default|GetPointsToControl)))))

(fn ResetArray
  (Variables|Default|SetPointsToControl (Utilities|Array|MakeArray 0 1 2 3)))

(fn GetAllSplineSegmentsLengths
  (params (In%20Spline :type Spline%20Component%20Object%20Reference))
  (bind _spline (Variables|Default|GetSpline))
  ;[1 1 1] Check if Input Spline is closed
  (if (Class|SplineComponent|IsClosedLoop In%20Spline)
    ;[1 1 1] Clear the map before execution
    (Utilities|Map|Clear (Variables|Default|GetSegment%20Lengths))
    (for _index (range 0 (SplineUtilities|GetSplineMaxIndex In%20Spline))
      ;[1 1 1] Initialize Local Variables
      (bind _output_get (LocalVariables|SetCurrentIndex _index))
      (LocalVariables|SetNextIndex (+ _output_get 1))
      ;[1 1 1] Check validity of input indices on spline
      (if (and (SplineUtilities|IsValidIndexonSpline (LocalVariables|GetCurrentIndex) _spline) (SplineUtilities|IsValidIndexonSpline (LocalVariables|GetNextIndex) _spline))
        ;[1 1 1] If Valid indices, add spline segments with associated points
        (Utilities|Map|Add (LocalVariables|GetLengths) (SplineSegments|GetSplineSegmentLength (LocalVariables|GetCurrentIndex) (LocalVariables|GetNextIndex) (Variables|Default|GetSpline)) (Utilities|Struct|MakeIntPoint (LocalVariables|GetCurrentIndex) (LocalVariables|GetNextIndex)))
        (else
          ;[1 1 1] Comment
          (if (> (LocalVariables|GetNextIndex) (SplineUtilities|GetSplineMaxIndex In%20Spline))
            ;[1 1 1] If the next index is not valid, add remaining segment to start
            (Utilities|Map|Add (LocalVariables|GetLengths) (SplineSegments|GetSplineSegmentLength (LocalVariables|GetCurrentIndex) 0 (Variables|Default|GetSpline)) (Utilities|Struct|MakeIntPoint (LocalVariables|GetCurrentIndex) 0))
            (else
              ;[1 1 1] If not valid, add impossible values
              (Utilities|Map|Add (LocalVariables|GetLengths) -1.0 (Utilities|Struct|MakeIntPoint -999 -999)))))))
    ;[1 1 1] Return the segment lengths and the associated Vertices
    (return (LocalVariables|GetLengths))))

(fn GetSplineSegmentLength
  (params (Index%20Start :type Integer) (Index%20End :type Integer) (Spline%20In :type Spline%20Component%20Object%20Reference))
  (if (and (SplineUtilities|IsValidIndexonSpline Index%20Start Spline%20In) (SplineUtilities|IsValidIndexonSpline Index%20End Spline%20In))
    (return (Math|Vector|Distance(Vector) (Spline|GetLocationatSplinePoint Spline%20In Index%20Start "Local") (Spline|GetLocationatSplinePoint Spline%20In Index%20End "Local")))
    (else
      (Development|PrintString "Index not Valid!"))))

(fn IsValidIndexonSpline
  (params (Index :type Integer) (Spline :type Spline%20Component%20Object%20Reference))
  (return (and (not (< Index 0)) (not (> Index (- (Spline|GetNumberOfSplinePoints Spline) 1))))))

(fn GetSplineMaxIndex
  (params (Target :type Spline%20Component%20Object%20Reference))
  (return (- (Spline|GetNumberOfSplinePoints Target) 1)))

(fn CalculateAreaOfTriangle
  (params (Index%20segment%20a :type Integer) (Index%20segment%20b :type Integer) (Index%20vertex%20diagonal%20a :type Integer) (Index%20vertex%20diagonal%20b :type Integer) (Length%20In :type Array%20of%20Floats%20%28double-precision%29) (Spline%20In :type Spline%20Component%20Object%20Reference))
  (Utilities|FlowControl|Sequence
    (:then_0
      ;[0.4349 1 0.7112] S = 1/2(a+b+c)
      ;;[1 1 1] Calculate Diagonal Length
      (LocalVariables|SetDiagonalLength (SplineSegments|GetSplineSegmentLength Index%20vertex%20diagonal%20a Index%20vertex%20diagonal%20b Spline%20In))
      ;;[1 1 1] s
      (LocalVariables|SetSemi-Perimeter (/ (+ (Utilities|Array|Get(acopy) Length%20In Index%20segment%20a) (Utilities|Array|Get(acopy) Length%20In Index%20segment%20b) (LocalVariables|GetDiagonalLength)) 2.0)))
    (:then_1
      ;[0.4349 1 0.7112] A = sq(s(s-a)(s-b)(s-c))
      (LocalVariables|SetArea (Math|Float|Sqrt (* (LocalVariables|GetSemi-Perimeter) (- (LocalVariables|GetSemi-Perimeter) (Utilities|Array|Get(acopy) Length%20In)) (- (LocalVariables|GetSemi-Perimeter) (Utilities|Array|Get(acopy) Length%20In 1)) (- (LocalVariables|GetSemi-Perimeter) (LocalVariables|GetDiagonalLength))))))
    (:then_2
      (return (LocalVariables|GetArea)))))

(fn ConvertLengthtoUnit
  (params (Unit :type E_MeasureUnits_Length%20Enum :default "NewEnumerator0") (Value :type Float%20%28double-precision%29))
  (return (Math|Conversions|ToFloat(Integer) (Units|AddUnitSuffix Unit (Utilities|Select :Index Unit :NewEnumerator0 (/ Value 1e+02) :NewEnumerator1 Value :NewEnumerator2 (* Value 1e+02) :NewEnumerator5 0.0 :NewEnumerator6 0.0 :NewEnumerator7 0.0)))))

(fn CalculateAreaOfIrregularQuadrilateral
  (params (In%20Spline :type Spline%20Component%20Object%20Reference) (SegmentLengths :type Array%20of%20Floats%20%28double-precision%29))
  (bind _triangle_area (HeronsFormula|CalculateAreaOfTriangle 0 1 0 2 (Variables|Default|GetSegmentLengths) In%20Spline))
  (bind _triangle_area_2 (HeronsFormula|CalculateAreaOfTriangle 2 3 0 2 (Variables|Default|GetSegmentLengths) In%20Spline))
  (return (Units|ConvertLengthtoUnit "NewEnumerator0" (/ (+ _triangle_area _triangle_area_2) 1e+02))))

(fn CalculateCenterPointOfClosedSpline
  (for _index (range 0 3)
    (Utilities|Array|Add (LocalVariables|GetLocations) (Spline|GetLocationatSplinePoint (Variables|Default|GetSpline) _index "World")))
  (return (Math|Vector|GetVectorArrayAverage (LocalVariables|GetLocations))))

(fn AddUnitSuffix
  (params (Unit :type E_MeasureUnits_Length%20Enum :default "NewEnumerator0") (Value :type Float%20%28double-precision%29))
  (return (Utilities|String|Append (Utilities|String|ToString(Float) Value) " " (Utilities|Select :Index Unit :NewEnumerator0 "m" :NewEnumerator1 "cm" :NewEnumerator2 "mm" :NewEnumerator5 "" :NewEnumerator6 "" :NewEnumerator7 ""))))

(fn ConvertSurfacetoUnit
  (params (Unit :type E_MeasureUnits_Surface%20Enum :default "NewEnumerator0") (Value :type Float%20%28double-precision%29))
  (return (Utilities|Select :Index Unit :NewEnumerator0 (/ Value 1e+02) :NewEnumerator5 Value :NewEnumerator1 (* Value 1e+02))))